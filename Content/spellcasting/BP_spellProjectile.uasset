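; Spell projectile actor that casts its spell type on any overlapped actor implementing spellable via TrySpell.
; BeginSpell sets type and two colours on a dynamic sprite material and Niagara effect, then launches the physics collider away from the player with test velocity.
; It is built for reuse: setup shows the collider, enables overlaps and marks it active, while EndSpell reverses this without destroying the actor.
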(event OnComponentBeginOverlap(collider)
  (params (OverlappedComponent :type Primitive%20Component%20Object%20Reference) (OtherActor :type Actor%20Object%20Reference) (OtherComp :type Primitive%20Component%20Object%20Reference) (OtherBodyIndex :type Integer) (bFromSweep :type Boolean) (SweepResult :type Hit%20Result%20Structure%20%28by%20ref%29))
  (bind _asspellable (Utilities|Casting|CastTospellable OtherActor))
  (Class|Spellable|TrySpell _asspellable (Variables|Default|GetspellType)))

(event EventBeginPlay
  (CallFunction|CreateMaterial))

(fn ConstructionScript)

(fn BeginSpell
  (params (spellType :type EspellType%20Enum :default "null") (colours :type 2colour%20Structure))
  (CallFunction|SetupSelf spellType colours)
  ;[0.15 0.15 0.15 0.5] testing
  (Physics|SetPhysicsLinearVelocity (Variables|Default|Getcollider) (* (Math|Vector|GetUnitDirection(Vector) (Transformation|GetActorLocation (Variables|Default|Getplayer)) (Transformation|GetActorLocation)) 5e+02) false "None"))

(fn EndSpell
  (Rendering|SetVisibility (Variables|Default|Getcollider) false true)
  (Variables|/Script/Engine.PrimitiveComponent|SetbGenerateOverlapEvents (Variables|Default|Getcollider) false)
  (Variables|Default|SetisActive false))

(fn CreateMaterial
  (bind _returnvalue (Rendering|Material|CreateDynamicMaterialInstance "/Game/spellcasting/aesthetics/spellCanvas.spellCanvas" "None" "None" :!class /Script/Engine.KismetMaterialLibrary))
  (Variables|Default|SetcanvasMaterial _returnvalue)
  (Rendering|Material|SetMaterial (Variables|Default|GetspritePlane) 0 (Variables|Default|GetcanvasMaterial)))

(fn SetupSelf
  (params (spellType :type EspellType%20Enum :default "null") (colours :type 2colour%20Structure))
  (bind (_colour1 _colour2) (Utilities|Struct|Break2colour colours))
  (Variables|Default|SetspellType spellType)
  (Rendering|Material|SetVectorParameterValue (Variables|Default|GetcanvasMaterial) "colour 1" _colour1 :!class /Script/Engine.MaterialInstanceDynamic)
  (Rendering|Material|SetVectorParameterValue (Variables|Default|GetcanvasMaterial) "colour 2" _colour2 :!class /Script/Engine.MaterialInstanceDynamic)
  (Niagara|SetNiagaraVariable(LinearColor) (Variables|Default|GetniagraTest2) "colour 1" _colour1)
  (Niagara|SetNiagaraVariable(LinearColor) (Variables|Default|GetniagraTest2) "colour 2" _colour2)
  (Rendering|SetVisibility (Variables|Default|Getcollider) true true)
  (Variables|/Script/Engine.PrimitiveComponent|SetbGenerateOverlapEvents (Variables|Default|Getcollider) true)
  (Physics|SetPhysicsLinearVelocity (Variables|Default|Getcollider) "0, 0, 0" false "None")
  (Variables|Default|SetisActive true))