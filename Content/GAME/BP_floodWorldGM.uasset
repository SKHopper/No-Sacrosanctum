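; BP_floodWorldGM is, by its name, the game mode for the flood world level and handles the player's entry into it.
; On BeginPlay it runs the parent logic, sets game-only input and hides the mouse cursor for the first player controller.
; It then creates a fade widget, adds it to the viewport and plays its fade-from-black animation.
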(event EventBeginPlay
  (bind _returnvalue (Game|GetPlayerController 0))
  (|CallParentFunction)
  (Input|SetInputModeGameOnly _returnvalue false)
  (Variables|/Script/Engine.PlayerController|SetbShowMouseCursor _returnvalue false)
  (bind _returnvalue_2 (UserInterface|CreateWidget "/Game/GAME/menu/fadeWidget.fadeWidget_C"))
  (UserInterface|Viewport|AddtoViewport _returnvalue_2 0)
  (Default|AnimFadefromBlack _returnvalue_2 true))

(event EventTick
  (params (DeltaSeconds :type Float%20%28single-precision%29))
  (|CallParentFunction DeltaSeconds) ; This node is disabled and will not be called.\nDrag off pins to build functionality.
)

(fn ConstructionScript
  (|CallParentFunction))