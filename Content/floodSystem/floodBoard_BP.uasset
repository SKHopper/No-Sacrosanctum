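; Flood board actor in the flood system that materializes into a solid board when its BoardUpEffect event fires.
; On BeginPlay it creates a dynamic material instance from BoardMaterial and applies it to the mesh.
; BoardUpEffect enables query and physics collision on GeneralCollider, then plays the Materialize timeline, which drives the material's "amount" parameter, clamped between zero and one.
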(event EventBoardUpEffect
  (Collision|SetCollisionEnabled (Variables|Default|GetgeneralCollider) "QueryAndPhysics")
  (bind _newtrack_0 (Timeline|materialize PlayFromStart)
    (:Update
      (Rendering|Material|SetScalarParameterValue (Variables|Default|Getmaterial) "amount" (Math|Float|Clamp(Float) _newtrack_0) :!class /Script/Engine.MaterialInstanceDynamic))))

(event EventBeginPlay
  (CallFunction|CreateMaterial))

(fn ConstructionScript)

(fn CreateMaterial
  (bind _returnvalue (Rendering|Material|CreateDynamicMaterialInstance "/Game/floodSystem/aesthetics/boardMaterial.boardMaterial" "None" "None" :!class /Script/Engine.KismetMaterialLibrary))
  (bind _output_get (Variables|Default|Setmaterial _returnvalue))
  (Rendering|Material|SetMaterial (Variables|Character|GetMesh) 0 _output_get))